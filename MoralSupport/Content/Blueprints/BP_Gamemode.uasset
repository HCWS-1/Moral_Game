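; BP_Gamemode is a game mode Blueprint that opens the main menu and manages switching between UI screens.
; On BeginPlay it creates WBP_MainMenu, adds it to the viewport and shows the mouse cursor.
; Its UpdateWidget event removes top-level widgets of the stored CurrentWidget class, stores the class passed in, then creates and displays that widget.
; BeginPlay does not set CurrentWidget for the initial menu.
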(event `self.ReceiveBeginPlay`
  (bind _returnvalue (`|CreateWidget` "/Game/Blueprints/Widgets/WBP_MainMenu.WBP_MainMenu_C"))
  (`UserWidget.AddToViewport` _returnvalue 0)
  (set `PlayerController.bShowMouseCursor` true (`GameplayStatics.GetPlayerController` 0)))

(event `UpdateWidget`
  (params (Widget :type "UserWidget Class Reference"))
  (bind _foundwidgets (`WidgetBlueprintLibrary.GetAllWidgetsOfClass` (`self.CurrentWidget`)))
  (`Widget.RemoveFromParent` _foundwidgets)
  (bind _output_get (set `self.CurrentWidget` Widget))
  (bind _returnvalue (`|CreateWidget` _output_get))
  (`UserWidget.AddToViewport` _returnvalue 0))

(fn `UserConstructionScript`)